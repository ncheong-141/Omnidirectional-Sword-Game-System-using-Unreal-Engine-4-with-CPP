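; NPC slash demonstrator that counts hits taken and destroys itself after enough of them.
; Tick narrows the capsule while blocking and uses an Incremented latch to count each HasBeenHit activation once, printing the total.
; At the hit threshold it sets Dead and runs a printed countdown to destruction, which pauses while HasBeenHit stays set.
; The hit and blocking flags are only read here.
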(event EventBeginPlay
  (Variables|Default|SetHitCounter 0.0)
  (Variables|Default|SetTimeTillDestroy 3.0))

(event Collision|EventActorBeginOverlap
  (params (OtherActor :type Actor%20Object%20Reference)))

(event EventTick
  (params (DeltaSeconds :type Float%20%28single-precision%29))
  (bind _capsulecomponent (Variables|Default|GetCapsuleComponent))
  (bind _hasbeenhit (Variables|Default|GethasBeenHit))
  (if (Variables|Default|GetisBlocking)
    (Components|Capsule|SetCapsuleRadius _capsulecomponent 15.0 true)
    (else
      (Components|Capsule|SetCapsuleRadius _capsulecomponent 34.0 true)))
  (if (and _hasbeenhit (not (Variables|Default|Getincremented)))
    (Variables|Default|Setincremented true)
    (bind _result (Math|Float|IncrementFloat (Variables|Default|GetHitCounter))
      (:%20%20
        (bind _output_get (Variables|Default|SetHitCounter _result))
        (Development|PrintString (Utilities|String|ToString(Float) _output_get))
        (if (>= _output_get 1e+02) :!label _label
          (bind _output_get_2 (Variables|Default|Setdead true))
          (if _output_get_2
            (bind _output_get_3 (Variables|Default|SetTimeTillDestroy (- (Variables|Default|GetTimeTillDestroy) DeltaSeconds)))
            (Development|PrintString (Utilities|String|ToString(Float) _output_get_3))
            (if (< _output_get_3 0.0)
              (Actor|DestroyActor))))))
    (elif (not _hasbeenhit)
      (Variables|Default|Setincremented false)
      (goto _label))))

(fn ConstructionScript)