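; Target dummy boss with a melee weapon that is destroyed after taking enough hits.
; Tick polls state flags, shrinking the capsule while blocking and playing sword clash or swing sounds at the weapon.
; Latch booleans make each sound and hit count register once per occurrence.
; Hits are counted only while its attack is neither blocked nor damaging; reaching the limit starts a per-tick countdown to DestroyActor.
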(event EventBeginPlay)

(event Collision|EventActorBeginOverlap
  (params (OtherActor :type Actor%20Object%20Reference)))

(event EventTick
  (params (DeltaSeconds :type Float%20%28single-precision%29))
  (bind _self self)
  (bind _capsulecomponent (Variables|Default|GetCapsuleComponent))
  (bind _wasblocked (Variables|Default|GetwasBlocked))
  (bind _hasbeenhit (Variables|Default|GethasBeenHit))
  (bind _meleeweapon (Variables|Default|GetMeleeWeapon _self))
  (if (Variables|Default|GetisBlocking)
    (Components|Capsule|SetCapsuleRadius _capsulecomponent 15.0 true)
    (else
      (Components|Capsule|SetCapsuleRadius _capsulecomponent 34.0 true)))
  (if (and _wasblocked (not (Variables|Default|GetPlayed%20sound?)))
    (Audio|PlaySoundatLocation "/Game/Music/SwordHitSword.SwordHitSword" (Transformation|GetActorLocation (Variables|Default|GetMeleeWeapon self)) "0, 0, 0" 1.0 1.0 0.0 0 0 0)
    (Variables|Default|SetPlayed%20sound? true))
  (if (not _wasblocked)
    (Variables|Default|SetPlayed%20sound? false)
    (Variables|Default|SetCan%20Damage (Variables|/Script/SwordPhysicsSystem.MeleeWeapon|GetcanDamage _meleeweapon))
    (if (and (Variables|Default|GetCan%20Damage) (not (Variables|Default|GetPlayed%20slash%20sound?)))
      (Audio|PlaySoundatLocation "/Game/Music/SwordWooshesHeavy.SwordWooshesHeavy" (Transformation|GetActorLocation _meleeweapon) "0, 0, 0" 1.0 1.0 0.0 0 0 0)
      (Variables|Default|SetPlayed%20slash%20sound? true))
    (if (not (Variables|Default|GetCan%20Damage))
      (Variables|Default|SetPlayed%20slash%20sound? false)
      (if (and _hasbeenhit (not (Variables|Default|Getincremented)))
        (Variables|Default|Setincremented true)
        (bind _result (Math|Float|IncrementFloat (Variables|Default|GetHitCounter))
          (:%20%20
            (bind _output_get (Variables|Default|SetHitCounter _result))
            (if (>= _output_get 25.0) :!label _label
              (bind _output_get_2 (Variables|Default|Setdead true))
              (if _output_get_2
                (bind _output_get_3 (Variables|Default|SetTimeTillDestroy (- (Variables|Default|GetTimeTillDestroy) 1.0)))
                (if (< _output_get_3 0.0)
                  (Actor|DestroyActor))))))
        (elif (not _hasbeenhit)
          (Variables|Default|Setincremented false)
          (goto _label))))))

(fn ConstructionScript)