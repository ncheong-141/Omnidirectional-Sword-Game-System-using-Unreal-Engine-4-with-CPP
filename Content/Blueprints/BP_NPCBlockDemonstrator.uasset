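; NPC that demonstrates melee blocking, built to destroy itself after five counted blocks.
; Tick polls the blocked flag and the melee weapon's damage window to play one-shot clash and slash sounds.
; The block counter check is nested in the not-blocked path; reaching the limit runs a printed countdown before destruction.
; Disconnected logic would shrink the capsule while blocking.
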(event EventBeginPlay
  (Variables|Default|SetBlockCounter 0.0)
  (Variables|Default|SetTimeTillDestroy 3.0))

(event Collision|EventActorBeginOverlap
  (params (OtherActor :type Actor%20Object%20Reference)))

(event EventTick
  (params (DeltaSeconds :type Float%20%28single-precision%29))
  (bind _wasblocked (Variables|Default|GetwasBlocked))
  ;[1 1 1] Sound
  (if (and _wasblocked (not (Variables|Default|GetPlayed%20sound?)))
    (Audio|PlaySoundatLocation "/Game/Music/SwordHitSword.SwordHitSword" (Transformation|GetActorLocation (Variables|Default|GetMeleeWeapon self)) "0, 0, 0" 1.0 1.0 0.0 0 0 0)
    (Variables|Default|SetPlayed%20sound? true))
  (if (not _wasblocked)
    (Variables|Default|SetPlayed%20sound? false)
    (Variables|Default|SetCan%20Damage (Variables|/Script/SwordPhysicsSystem.MeleeWeapon|GetcanDamage (Variables|Default|GetMeleeWeapon self)))
    (if (and (Variables|Default|GetCan%20Damage) (not (Variables|Default|GetPlayed%20slash%20sound?)))
      (Audio|PlaySoundatLocation "/Game/Music/SwordWooshesLight.SwordWooshesLight" (Transformation|GetActorLocation) "0, 0, 0" 1.0 1.0 0.0 0 0 0)
      (Variables|Default|SetPlayed%20slash%20sound? true)
      (if (and (Variables|Default|GetwasBlocked) (not (Variables|Default|GetCounted?))) :!label _label
        (Variables|Default|SetCounted? true)
        (bind _result (Math|Float|IncrementFloat (Variables|Default|GetBlockCounter))
          (:%20%20
            (bind _output_get (Variables|Default|SetBlockCounter _result))
            (if (>= _output_get 5.0)
              (bind _output_get_2 (Variables|Default|Setdead (>= _output_get 5.0) :!label _label_2))
              (if _output_get_2
                (bind _output_get_3 (Variables|Default|SetTimeTillDestroy (- (Variables|Default|GetTimeTillDestroy) DeltaSeconds)))
                (Development|PrintString (Utilities|String|ToString(Float) _output_get_3))
                (if (< _output_get_3 0.0)
                  (Actor|DestroyActor))))))
        (else
          (Variables|Default|SetCounted? false)
          (goto _label_2)))
      (elif (not (Variables|Default|GetCan%20Damage))
        (Variables|Default|SetPlayed%20slash%20sound? false)
        (goto _label)))))

(fn ConstructionScript)